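; BP_TestBlock is a test item block meant as a template for custom pickup logic, though it currently does nothing.
; Its Pickup event is empty, and the node chain for pickup is disconnected.
; That unused chain would add a visible block to BP_PlayerCharacter's ItemArray, store the index, then hide it and disable collision instead of destroying it.
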(event `/Game/GEP/Blueprints/Interfaces/BPI_Pickupable.Pickup`
  ;[0.8879 0.2346 0.2346] This is where you will want to add your own implementation for your own systems. Checks if item is visible, if so it appends it to array and then makes it invisible
)

(fn `UserConstructionScript`)