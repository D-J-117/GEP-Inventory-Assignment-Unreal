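; BP_ExampleItem is an example pickup item actor, meant as a starting point for custom item systems.
; On BeginPlay, an ID of 2 gives its mesh a blue material.
; Pickup, if the mesh is visible, adds the item to BP_PlayerCharacter's ItemArray, stores the index, then hides the Sphere hierarchy and disables collision.
; DropItem restores visibility and collision without removing the array entry, so the actor is reused rather than destroyed.
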(event `self.ReceiveBeginPlay`
  (if (== (`self.ID`) 2)
    (`PrimitiveComponent.SetMaterial` (`self.Mesh`) 0 "/Game/LevelPrototyping/Materials/MI_Solid_Blue.MI_Solid_Blue")))

(event `/Game/GEP/Blueprints/Interfaces/BPI_Pickupable.Pickup`
  ;[0.8879 0.2346 0.2346] This is where you will want to add your own implementation for your own systems. Checks if item is visible, if so it appends it to array and then makes it invisible
  (if (`SceneComponent.IsVisible` (`self.Mesh`))
    (bind _asbp_player_character (cast `/Game/GEP/Blueprints/Essentials/BP_PlayerCharacter` (`GameplayStatics.GetPlayerCharacter` 0)))
    (bind _returnvalue (`KismetArrayLibrary.Array_Add` (`/Game/GEP/Blueprints/Essentials/BP_PlayerCharacter.Item_Array` _asbp_player_character) self))
    (set `self.Array_Index` _returnvalue)
    (`SceneComponent.SetVisibility` (`self.Sphere`) false true)
    (`self.SetActorEnableCollision` self false)))

(event `Drop Item`
  (`SceneComponent.SetVisibility` (`self.Sphere`) true true)
  (`self.SetActorEnableCollision` self true))

(fn `UserConstructionScript`)